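; BP_Player is the Crossy Road style chicken player, which hops along a grid and handles its own deaths.
; A held axis stores one step on a single axis, and releasing it triggers a swept hop.
; Overlapping a non-log BP_Car flattens the mesh as a crash or squish, depending on the sweep flag.
; Drown and fall-out functions add a splash or eagle, and every death calls Defeat to signal PlayerDied.
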(event `self.Chicken.OnComponentBeginOverlap`
  (params (OverlappedComponent :type "PrimitiveComponent Object Reference") (OtherActor :type "Actor Object Reference") (OtherComp :type "PrimitiveComponent Object Reference") (OtherBodyIndex :type Integer) (bFromSweep :type Boolean) (SweepResult :type "HitResult Structure (by ref)"))
  (if (not (`self.Dead`))
    (bind _asbp_car (cast `/Game/CrossyRoad/Blueprints/BP_Car` OtherActor))
    (cast `/Game/CrossyRoad/Blueprints/BP_Log` _asbp_car
      (:`CastFailed`
        (if bFromSweep
          (`self.ChickenCrash`)
          (else
            (`self.ChickenSquish`)))))))

(event `InputAxis|MoveForward`
  (params (AxisValue :type "Float (single-precision)"))
  (if (`KismetMathLibrary.NearlyEqual_FloatFloat` AxisValue 0.0 0.001)
    (if (`self.InputX`)
      (`self.Hop`))
    (elif (not (`self.InputY`))
      (set `self.HeldInput` (`KismetMathLibrary.MakeVector` (* AxisValue 80.0)))
      (set `self.InputX` true))))

(event `InputAxis|MoveRight`
  (params (AxisValue :type "Float (single-precision)"))
  (if (`KismetMathLibrary.NearlyEqual_FloatFloat` AxisValue 0.0 0.001)
    (if (`self.InputY`)
      (`self.Hop`))
    (elif (not (`self.InputX`))
      (set `self.HeldInput` (`KismetMathLibrary.MakeVector` 0.0 (* AxisValue 80.0)))
      (set `self.InputY` true))))

(fn `ChickenCrash`
  (bind _chickenmesh (`self.ChickenMesh`))
  (`SceneComponent.K2_SetRelativeLocation` _chickenmesh (-45.0 0.0 -5.0) false false)
  (`SceneComponent.SetRelativeScale3D` _chickenmesh (0.1 0.4 0.4))
  (`self.Defeat`))

(fn `ChickenDrown`
  (`ActorComponent.K2_DestroyComponent` (`self.Chicken`))
  (`ActorComponent.K2_DestroyComponent` (`self.ChickenMesh`))
  (bind _returnvalue (`AddComponent|NODE_AddNiagaraComponent-3`))
  (`FXSystemComponent.SetEmitterEnable` _returnvalue "Splash" true)
  (`self.Defeat`))

(fn `ChickenSquish`
  (bind _chickenmesh (`self.ChickenMesh`))
  (`SceneComponent.K2_SetRelativeLocation` _chickenmesh (0.0 0.0 -35.0) false false)
  (`SceneComponent.SetRelativeScale3D` _chickenmesh (0.4 0.4 0.1))
  (`self.Defeat`))

(fn `Defeat`
  (set `self.Dead` true)
  (`self.PlayerDied`))

(fn `FallOut`
  (`|SpawnActorFromClass` "/Game/CrossyRoad/Blueprints/BP_Eagle.BP_Eagle_C" (`KismetMathLibrary.MakeTransform` (1200.0 200.0 200.0)) "Undefined" "OverrideRootScale" null null)
  (`self.Defeat`))

(fn `Hop`
  (bind (_heldinput_x _heldinput_y) (`KismetMathLibrary.BreakVector` (`self.HeldInput`)))
  (if (not (`self.Dead`))
    (`SceneComponent.K2_SetWorldRotation` (`self.ChickenMesh`) (`KismetMathLibrary.Conv_VectorToRotator` (`self.HeldInput`)) false false)
    (`SceneComponent.K2_AddLocalOffset` (`self.Chicken`) (`KismetMathLibrary.MakeVector` _heldinput_x _heldinput_y 5.0) true false)
    (set `self.HeldInput` (0.0 0.0 0.0))
    (set `self.InputX` false)
    (set `self.InputY` false)))

(fn `UserConstructionScript`)