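; Lane spawner for a Crossy Road-style game that builds the starting strip of BP_Lane actors and keeps it scrolling.
; At BeginPlay it replaces existing lanes, starting with grass-only ones, and registers with the game mode.
; Lanes form a linked list: each timed step appends one, destroys the oldest and offsets the player along local X.
; The step interval shrinks as LanesPassed grows, down to a fixed minimum.
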(event `self.ReceiveBeginPlay`
  (`self.SpawnInitialLanes`)
  (bind _asbp_crossy_road (cast `/Game/CrossyRoad/Blueprints/BP_CrossyRoad` (`GameplayStatics.GetGameMode`)))
  (set `/Game/CrossyRoad/Blueprints/BP_CrossyRoad.Spawner` self _asbp_crossy_road))

(event `self.ReceiveTick`
  (params (DeltaSeconds :type "Float (single-precision)"))
  (bind _output_get (set `self.TimePassed` (+ DeltaSeconds (`self.TimePassed`))))
  (if (>= _output_get (`KismetMathLibrary.FClamp` (- 3.0 (* (`self.LanesPassed`) 0.02)) 0.8 3.0))
    (set `self.TimePassed` 0.0)
    (`self.SpawnNextLane` false true)))

(fn `SpawnInitialLanes`
  (`|ExecutionSequence`
    (:`then_0`
      (bind _outactors (`GameplayStatics.GetAllActorsOfClass` "/Game/CrossyRoad/Blueprints/BP_Lane.BP_Lane_C"))
      (for _array_element _outactors
        (`self.K2_DestroyActor` _array_element)))
    (:`then_1`
      (for _index (range (+ (`self.InitialLaneCount`) 1))
        (`/Engine/EditorBlueprintResources/StandardMacros.IsValid` (`self.NewestLane`)
          (:`Is Valid`
            (`self.SpawnNextLane` (<= _index (`self.GrassLanes`))))
          (:`Is Not Valid`
            (bind _newlane (`self.SpawnLane` (`SceneComponent.K2_GetComponentLocation` (`self.DefaultSceneRoot`))))
            (set `self.OldestLane` _newlane)))))))

(fn `SpawnLane`
  (params (Position :type "Vector Structure"))
  (returns (NewLane :type "/Game/CrossyRoad/Blueprints/BP_Lane Object Reference"))
  (bind _newestlane (`self.NewestLane`))
  (bind _returnvalue (`|SpawnActorFromClass` "/Game/CrossyRoad/Blueprints/BP_Lane.BP_Lane_C" (`KismetMathLibrary.MakeTransform` Position) "Undefined" "OverrideRootScale" null null))
  (if (`KismetSystemLibrary.IsValid` _newestlane)
    (bind _output_get (set `self.PreviousLane` _newestlane))
    (set `/Game/CrossyRoad/Blueprints/BP_Lane.NextLane` _returnvalue _output_get))
  (bind _output_get_2 (set `self.NewestLane` _returnvalue))
  (set `/Game/CrossyRoad/Blueprints/BP_Lane.Spawner` self _output_get_2)
  (return _returnvalue))

(fn `SpawnNextLane`
  (params (GrassOnly :type Boolean) (RemoveLast :type Boolean))
  (locals (NextOldLane :type "/Game/CrossyRoad/Blueprints/BP_Lane Object Reference"))
  (bind _oldestlane (`self.OldestLane`))
  (bind _newlane (`self.SpawnLane` (`SceneComponent.K2_GetComponentLocation` (`/Game/CrossyRoad/Blueprints/BP_Lane.SpawnPoint` (`self.NewestLane`)))))
  (`/Game/CrossyRoad/Blueprints/BP_Lane.Setup Lane Mesh` _newlane GrassOnly)
  (if RemoveLast
    (set `local.NextOldLane` (`/Game/CrossyRoad/Blueprints/BP_Lane.NextLane` _oldestlane))
    (`/Game/CrossyRoad/Blueprints/BP_Lane.DestroyLane` _oldestlane)
    (set `self.OldestLane` (`local.NextOldLane`))
    (bind _asbp_player (cast `/Game/CrossyRoad/Blueprints/BP_Player` (`GameplayStatics.GetPlayerPawn` 0)))
    (`SceneComponent.K2_AddLocalOffset` (`Actor.RootComponent` _asbp_player) (80.0 0.0 0.0) false false)))

(fn `UserConstructionScript`)