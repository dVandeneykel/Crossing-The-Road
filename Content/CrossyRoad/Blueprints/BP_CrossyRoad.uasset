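; BP_CrossyRoad is the manager for the Crossy Road game, linking lane-crossing progress to the HUD.
; On BeginPlay it binds to the Spawner's lane-passed event, then creates BP_HUD, hands itself over as Manager and has the HUD subscribe to updates.
; Each crossed lane copies the Spawner's LanesPassed count and fires the PlayerCrossedLane dispatcher.
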(event `LaneCrossed`
  (set `self.LanesPassed` (`/Game/CrossyRoad/Blueprints/BP_LaneSpawner.LanesPassed` (`self.Spawner`)))
  (`self.PlayerCrossedLane`))

(event `self.ReceiveBeginPlay`
  (`|ExecutionSequence`
    (:`then_0`
      (add `/Game/CrossyRoad/Blueprints/BP_LaneSpawner.LaneWasPassed` (`self.Spawner`) (delegate `LaneCrossed`)))
    (:`then_1`
      (bind _returnvalue (`|GenericCreateObject` "/Game/CrossyRoad/Blueprints/BP_HUD.BP_HUD_C"))
      (`UserWidget.AddToViewport` _returnvalue 0)
      (set `/Game/CrossyRoad/Blueprints/BP_HUD.Manager` self _returnvalue)
      (`/Game/CrossyRoad/Blueprints/BP_HUD.SubscribeUpdate` _returnvalue))))

(fn `UserConstructionScript`)