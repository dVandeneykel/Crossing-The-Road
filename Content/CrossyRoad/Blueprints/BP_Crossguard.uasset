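; BP_Crossguard is a crossing signal in the CrossyRoad game that flashes two lights alternately while signaling is active.
; StartSignal lights the first lamp and enables signaling, and EndSignal stops it and switches both lamps off.
; While signaling, Tick accumulates time and calls AdjustSignalColor at a fixed short interval.
; AdjustSignalColor swaps on and off materials between the lamps and toggles the LeftSignal flag.
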(event `self.ReceiveTick`
  (params (DeltaSeconds :type "Float (single-precision)"))
  (if (`self.Signaling`)
    (bind _output_get (set `self.Time` (+ DeltaSeconds (`self.Time`))))
    (if (>= _output_get 0.4)
      (`self.AdjustSignalColor`)
      (set `self.Time` 0.0))))

(fn `AdjustSignalColor`
  (bind _light1 (`self.Light1`))
  (bind _light2 (`self.Light2`))
  (if (`self.LeftSignal`)
    (`PrimitiveComponent.SetMaterial` _light1 0 "/Game/CrossyRoad/Models/LightOn.LightOn")
    (`PrimitiveComponent.SetMaterial` _light2 0 "/Game/CrossyRoad/Models/LightOff.LightOff")
    (else
      (`PrimitiveComponent.SetMaterial` _light1 0 "/Game/CrossyRoad/Models/LightOff.LightOff")
      (`PrimitiveComponent.SetMaterial` _light2 0 "/Game/CrossyRoad/Models/LightOn.LightOn")))
  (set `self.LeftSignal` (not (`self.LeftSignal`)))
  (return))

(fn `EndSignal`
  (set `self.Signaling` false)
  (`PrimitiveComponent.SetMaterial` (`self.Light1`) 0 "/Game/CrossyRoad/Models/LightOff.LightOff")
  (`PrimitiveComponent.SetMaterial` (`self.Light2`) 0 "/Game/CrossyRoad/Models/LightOff.LightOff"))

(fn `StartSignal`
  (set `self.Signaling` true)
  (set `self.Time` 0.0)
  (`PrimitiveComponent.SetMaterial` (`self.Light1`) 0 "/Game/CrossyRoad/Models/LightOn.LightOn"))

(fn `UserConstructionScript`)